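; BP_CameraVectorOrientation is a Shader Museum exhibit actor that shows how a camera's forward vector changes as it rotates.
; Each tick it yaws the Camera component in world space by Speed scaled by delta time.
; It then reads the forward vector, rounds each axis to one decimal and writes the X, Y and Z values to a TextRender component.
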(event EventTick
  (params (DeltaSeconds :type Float%20%28single-precision%29))
  (Transformation|AddWorldRotation (Variables|Default|GetCamera) (Math|Rotator|MakeRotator 0.0 0.0 (* DeltaSeconds (Variables|Default|GetSpeed))) false false)
  (bind _output_get (Variables|Default|SetVector%20Value (Math|Vector|GetForwardVector (Variables|Default|GetCamera))))
  (Rendering|Components|TextRender|SetText (Variables|Default|GetTextRender) (Utilities|Text|ToText(String) (Utilities|String|Append "(X =" (Utilities|String|ToString(Float) (* (Math|Conversions|ToFloat(Integer) (Math|Float|Round (* (.X (Math|Vector|BreakVector _output_get)) 1e+01))) 0.1)) "; Y = " (Utilities|String|ToString(Float) (* (Math|Conversions|ToFloat(Integer) (Math|Float|Round (* (.Y (Math|Vector|BreakVector _output_get)) 1e+01))) 0.1)) "; Z = " (Utilities|String|ToString(Float) (* (Math|Conversions|ToFloat(Integer) (Math|Float|Round (* (.Z (Math|Vector|BreakVector _output_get)) 1e+01))) 0.1)) ")"))))

(fn ConstructionScript)